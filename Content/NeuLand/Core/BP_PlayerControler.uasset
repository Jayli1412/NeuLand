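; Player controller that relays movement, camera look and jump input to the possessed BP_HoRut pawn.
; Each axis or action event casts the controlled pawn to BP_HoRut and calls its matching function, doing nothing if the cast fails.
; Jump press and release call separate start and stop functions, so the pawn itself holds all movement logic.
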(event `InputAxis|Move Forward/Backward`
  (params (AxisValue :type "Float (single-precision)"))
  ;[0 1 0.01562] Move Control
  (bind _asbp_ho_rut (cast `/Game/NeuLand/Characters/BP_HoRut` (`self.K2_GetPawn`)))
  (`/Game/NeuLand/Characters/BP_HoRut.MoveForward/Backward` _asbp_ho_rut AxisValue))

(event `InputAxis|Move Left/Right`
  (params (AxisValue :type "Float (single-precision)"))
  ;[0 1 0.01562] Move Control
  (bind _asbp_ho_rut (cast `/Game/NeuLand/Characters/BP_HoRut` (`self.K2_GetPawn`)))
  (`/Game/NeuLand/Characters/BP_HoRut.MoveLeft/Right` _asbp_ho_rut AxisValue))

(event `InputAxis|LookAround`
  (params (AxisValue :type "Float (single-precision)"))
  ;[1 0.7969 0] Look Control
  (bind _asbp_ho_rut (cast `/Game/NeuLand/Characters/BP_HoRut` (`self.K2_GetPawn`)))
  (`/Game/NeuLand/Characters/BP_HoRut.LookAround` _asbp_ho_rut AxisValue))

(event `InputAxis|LookUp/Down`
  (params (AxisValue :type "Float (single-precision)"))
  ;[1 0.7969 0] Look Control
  (bind _asbp_ho_rut (cast `/Game/NeuLand/Characters/BP_HoRut` (`self.K2_GetPawn`)))
  (`/Game/NeuLand/Characters/BP_HoRut.LookUpDown` _asbp_ho_rut AxisValue))

(event `InputAction|Jump`
  (params (Key :type "Key Structure"))
  (bind _returnvalue (`self.K2_GetPawn`))
  ;[1 0.1875 0] Jump Control
  (:`Pressed`
    (bind _asbp_ho_rut (cast `/Game/NeuLand/Characters/BP_HoRut` _returnvalue))
    (`/Game/NeuLand/Characters/BP_HoRut.Juuump` _asbp_ho_rut))
  (:`Released`
    (bind _asbp_ho_rut_2 (cast `/Game/NeuLand/Characters/BP_HoRut` _returnvalue))
    (`/Game/NeuLand/Characters/BP_HoRut.NoJump` _asbp_ho_rut_2)))

(fn `UserConstructionScript`)